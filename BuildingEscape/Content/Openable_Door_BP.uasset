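; Openable door actor that swings open and closed by rotating around its vertical axis.
; An open event plays a timeline whose yaw curve is combined with the rotation cached at BeginPlay, so the swing is relative to the door's placement.
; A timeline event track plays a door lock sound at the actor's location, and the close event reverses the same timeline.
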(event `self.OpenDoor.OnOpen`
  (bind (_direction _open_angle) (`Timeline|Timeline_0` :!label _label)
    (:`Update`
      (`self.K2_SetActorRotation` (`KismetMathLibrary.ComposeRotators` (`KismetMathLibrary.MakeRotator` 0.0 0.0 _open_angle) (`self.InitialRotation`))))
    (:`Sound Timing`
      (`GameplayStatics.PlaySoundAtLocation` "/Game/Audio/door-lock.door-lock" (`self.K2_GetActorLocation`)))))

(event `self.OpenDoor.OnClose`
  (goto _label :!via `Reverse`))

(event `self.ReceiveBeginPlay`
  (set `self.InitialRotation` (`self.K2_GetActorRotation`)))

(fn `UserConstructionScript`)